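; BP_Elevator is an actor that moves its Cube component up and down continuously as an elevator.
; BeginPlay calls TurnElevatorOn, which starts the raise cycle.
; Raise and Lower timelines scale their curve output to set the cube's relative Z, one playing forward and the other in reverse.
; Each timeline's Finished event triggers the other movement, forming an endless loop with no player trigger.
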(event `self.ReceiveBeginPlay`
  (`self.Turn Elevator On`))

(event `ElevatorRaise`
  (bind (_direction _raise_) (`Timeline|Raise` :!via `PlayFromStart`)
    (:`Update`
      (`SceneComponent.K2_SetRelativeLocation` (`self.Cube`) (`KismetMathLibrary.MakeVector` 0.0 0.0 (* _raise_ 2000.0)) false false))
    (:`Finished`
      (`self.ElevatorLower`))))

(event `ElevatorLower`
  (bind (_direction _raise_) (`Timeline|Lower` :!via `ReverseFromEnd`)
    (:`Update`
      (`SceneComponent.K2_SetRelativeLocation` (`self.Cube`) (`KismetMathLibrary.MakeVector` 0.0 0.0 (* _raise_ 2000.0)) false false))
    (:`Finished`
      (`self.ElevatorRaise`))))

(event `Turn Elevator On`
  (`self.ElevatorRaise`))

(fn `UserConstructionScript`)